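; BP_AudioPlayer is an audio-reactive actor that plays a sound and visualizes its loudness through a scaling mesh and a glowing sphere.
; BeginPlay binds the audio playback events, gives the sphere a dynamic red-light material, then starts playback after a short delay.
; Each playback update reads the cooked envelope data to drive the mesh's Z scale and the material's emissive intensity, both zeroed when the audio finishes.
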(event `self.ReceiveBeginPlay`
  (bind _audio (`self.Audio`))
  (add `AudioComponent.OnAudioPlaybackPercent` _audio (delegate `OnAudioPlayback`))
  (add `AudioComponent.OnAudioFinished` _audio (delegate `OnAudioFinished`))
  (bind _returnvalue (`KismetMaterialLibrary.CreateDynamicMaterialInstance` "/Game/Audio/MI_RedLight.MI_RedLight"))
  (set `self.Dynamic Material Lights` _returnvalue)
  (`PrimitiveComponent.SetMaterial` (`self.Sphere`) 0 (`self.Dynamic Material Lights`))
  (`KismetSystemLibrary.Delay` 4.0)
  (`AudioComponent.Play` (`self.Audio`) 0.0))

(event `OnAudioPlayback`
  (params (PlayingSoundWave :type "SoundWave Object Reference") (PlaybackPercent :type "Float (single-precision)"))
  (bind _outenvelopedata (`AudioComponent.GetCookedEnvelopeData` (`self.Audio`)))
  (`SceneComponent.SetRelativeScale3D` (`self.StaticMesh`) (`KismetMathLibrary.MakeVector` 1.0 1.0 (* _outenvelopedata 10.0)))
  (`MaterialInstanceDynamic.SetScalarParameterValue` (`self.Dynamic Material Lights`) "Emissive" (* _outenvelopedata 4.0)))

(event `OnAudioFinished`
  (`SceneComponent.SetRelativeScale3D` (`self.StaticMesh`) (1.0 1.0 0.0))
  (`MaterialInstanceDynamic.SetScalarParameterValue` (`self.Dynamic Material Lights`) "Emissive" 0.0))

(fn `UserConstructionScript`)