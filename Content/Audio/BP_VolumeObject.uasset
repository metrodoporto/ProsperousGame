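; BP_VolumeObject is a speaker actor whose size is raised or lowered through AddVolume and SubVolume events.
; The construction script picks the speaker mesh and material from Width and Height.
; BeginPlay stores the starting scale and applies a dynamic material with its volume parameter at full.
; The events shift GoalSize within MinSize and MaxSize checks, and Tick steps the uniform scale toward it after a tiny Delay.
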(event `self.ReceiveBeginPlay`
  (bind _returnvalue_x (`KismetMathLibrary.BreakVector` (`self.GetActorScale3D`)))
  (set `self.goalSize` _returnvalue_x)
  (bind _returnvalue (`KismetMaterialLibrary.CreateDynamicMaterialInstance` (`PrimitiveComponent.GetMaterial` (`self.Speaker`) 0)))
  (`MaterialInstanceDynamic.SetScalarParameterValue` _returnvalue "volume" 1.0)
  (`PrimitiveComponent.SetMaterial` (`self.Speaker`) 0 _returnvalue))

(event `self.ReceiveTick`
  (params (DeltaSeconds :type "Float (single-precision)"))
  (bind _returnvalue_x (`KismetMathLibrary.BreakVector` (`self.GetActorScale3D`)))
  (bind _goalsize (`self.goalSize`))
  (bind _returnvalue (+ _returnvalue_x (`KismetMathLibrary.SelectFloat` 0.01 -0.01 (< _returnvalue_x _goalsize))))
  (`KismetSystemLibrary.Delay` 0.002)
  (if (!= _returnvalue_x _goalsize)
    (`self.SetActorScale3D` (`KismetMathLibrary.MakeVector` _returnvalue _returnvalue _returnvalue))))

(event `/Game/Interfaces/BPI_VolumeControled.addVolume`
  (bind _returnvalue_x (`KismetMathLibrary.BreakVector` (`self.GetActorScale3D`)))
  (if (< _returnvalue_x (`self.maxSize`))
    (set `self.goalSize` (+ _returnvalue_x 0.1))))

(event `/Game/Interfaces/BPI_VolumeControled.subVolume`
  (bind _returnvalue_x (`KismetMathLibrary.BreakVector` (`self.GetActorScale3D`)))
  (if (> _returnvalue_x (`self.minSize`))
    (set `self.goalSize` (- _returnvalue_x 0.1))))

(fn `UserConstructionScript`
  (bind _speaker (`self.Speaker`))
  (bind _returnvalue (- (+ (`self.Width`) (* (`self.Height`) 2)) 3))
  (`StaticMeshComponent.SetStaticMesh` _speaker (select `int` _returnvalue :`0` "/Game/Models/Speakers/speaker1x1.speaker1x1" :`1` "/Game/Models/Speakers/speaker2x1.speaker2x1" :`2` "/Game/Models/Speakers/speaker1x2.speaker1x2" :`3` null :!type "StaticMesh Object Reference"))
  (`PrimitiveComponent.SetMaterial` _speaker 0 (select `int` _returnvalue :`0` "/Game/Models/Speakers/MAT_speaker1x1.MAT_speaker1x1" :`1` "/Game/Models/Speakers/MAT_speaker2x1.MAT_speaker2x1" :`2` "/Game/Models/Speakers/MAT_speaker1x2.MAT_speaker1x2" :`3` null :!type "MaterialInterface Object Reference")))