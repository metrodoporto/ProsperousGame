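; BP_ChannelZone is a box trigger that changes the player's channel signal while their character is inside it.
; On entry it resets channels on BP_LevelCore and sends ChannelAmmount to PC_Player.
; On exit it sends a signal of 1 and has the core send a channel message.
; If no core exists at BeginPlay, it logs, destroys itself and switches every BP_channelObject according to the active channel.
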(event `self.ReceiveBeginPlay`
  (set `self.Player` (cast `/Game/Core/PC_Player` (`GameplayStatics.GetPlayerController` 0) :!pure true))
  (bind _returnvalue (`GameplayStatics.GetActorOfClass` "/Game/Blueprints/BP_LevelCore.BP_LevelCore_C"))
  (`/Engine/EditorBlueprintResources/StandardMacros.IsValid` _returnvalue
    (:`Is Valid`
      (set `self.Core` _returnvalue))
    (:`Is Not Valid`
      (`KismetSystemLibrary.PrintString` "Missing 'LevelCore' [BP_ChannelZone]")
      (`self.K2_DestroyActor`)
      (bind _outactors (`GameplayStatics.GetAllActorsOfClass` "/Game/Blueprints/Objects/BP_channelObject.BP_channelObject_C"))
      (for _array_element _outactors
        (`/Game/Blueprints/Objects/BP_channelObject.switchMe` _array_element (== (`/Game/Blueprints/Objects/BP_channelObject.Channel` _array_element) (`/Game/Core/PC_Player.activeChannel` (cast `/Game/Core/PC_Player` (`GameplayStatics.GetPlayerController` 0) :!pure true))))))))

(event `self.Box.OnComponentBeginOverlap`
  (params (OverlappedComponent :type "PrimitiveComponent Object Reference") (OtherActor :type "Actor Object Reference") (OtherComp :type "PrimitiveComponent Object Reference") (OtherBodyIndex :type Integer) (bFromSweep :type Boolean) (SweepResult :type "HitResult Structure (by ref)"))
  (if (== OtherActor (`GameplayStatics.GetPlayerCharacter` 0))
    (`/Game/Blueprints/BP_LevelCore.Channel Reset` (`self.Core`))
    (`/Game/Core/PC_Player.sendSignal` (`self.Player`) (`self.Channel Ammount`))))

(event `self.Box.OnComponentEndOverlap`
  (params (OverlappedComponent :type "PrimitiveComponent Object Reference") (OtherActor :type "Actor Object Reference") (OtherComp :type "PrimitiveComponent Object Reference") (OtherBodyIndex :type Integer))
  (if (== OtherActor (`GameplayStatics.GetPlayerCharacter` 0))
    (`/Game/Core/PC_Player.sendSignal` (`self.Player`) 1)
    (`/Game/Blueprints/BP_LevelCore.sendChannelMessage` (`self.Core`) true)))

(fn `UserConstructionScript`)