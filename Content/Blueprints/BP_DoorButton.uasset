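; Interactable door button Blueprint that, on interaction, tells a referenced actor to swap elevators, then open its doors after a short delay.
; A separate OpenDoor event, not triggered by OnInteract, raises an actor on one timeline, pauses, then lowers it on another.
; An AbleOpen flag blocks retriggering during that cycle, and movement adds timeline-scaled offsets to the current location each update.
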(event `self.ReceiveBeginPlay`)

(event `OpenDoor`
  (bind _actor (`self.Actor`))
  (bind _actor_2 (`self.Actor`))
  (if (`self.ableOpen`)
    (set `self.ableOpen` false)
    (bind (_direction _z) (`Timeline|Scaler` :!via `PlayFromStart`)
      (:`Update`
        (`self.K2_SetActorLocation` _actor_2 (+ (`self.K2_GetActorLocation` _actor_2) (`KismetMathLibrary.MakeVector` 0.0 0.0 (* _z 50.0))) false false))
      (:`Finished`
        (`KismetSystemLibrary.Delay` 3.0)
        (bind (_direction_2 _z_2) (`Timeline|Timeline` :!via `PlayFromStart`)
          (:`Update`
            (`self.K2_SetActorLocation` _actor (+ (`self.K2_GetActorLocation` _actor) (`KismetMathLibrary.MakeVector` 0.0 0.0 (* _z_2 -50.0))) false false))
          (:`Finished`
            (set `self.ableOpen` true)))))))

(event `/Game/Interfaces/Int_Interactable.onInteract`
  (params (Component :type "PrimitiveComponent Object Reference"))
  (bind _actor (`self.Actor`))
  (`/Game/Blueprints/BP_Elevator.swapElevators` _actor)
  (`KismetSystemLibrary.Delay` 1.0)
  (`/Game/Blueprints/BP_Elevator.openDoors` _actor))

(fn `UserConstructionScript`)