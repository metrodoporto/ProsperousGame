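; BP_Elevator is a fake elevator that teleports the player to a linked elevator, with sliding doors driven by the DoorAnim timeline.
; Entering the trigger closes both cars' doors after a delay, then moves the player to CurrentConnection, preserving their offset from the base.
; An OnTeleport flag makes the destination open its doors on arrival instead of sending the player back.
; SwapElevators exchanges current and alternate connections; closeALLDoors shuts every elevator.
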(event `self.ReceiveBeginPlay`
  (`self.openDoors`))

(event `closeALLDoors`
  (bind _outactors (`GameplayStatics.GetAllActorsOfClass` "BP_Elevator_C"))
  (for _array_element _outactors
    (`self.closeDoors` _array_element)))

(event `openDoors`
  (bind (_direction _difference) (`Timeline|DoorAnim` :!via `PlayFromStart` :!label _label)
    (:`Update`
      (bind _returnvalue (* _difference 80.0))
      (`SceneComponent.K2_SetRelativeLocation` (`self.DoorL`) (`KismetMathLibrary.MakeVector` (+ (* _returnvalue -1.0) -50.5) 120.0 200.0) false false)
      (`SceneComponent.K2_SetRelativeLocation` (`self.DoorR`) (`KismetMathLibrary.MakeVector` (+ _returnvalue 50.5) 120.0 200.0) false false))))

(event `closeDoors`
  (goto _label :!via `ReverseFromEnd`))

(event `self.insideElevator.OnComponentBeginOverlap`
  (params (OverlappedComponent :type "PrimitiveComponent Object Reference") (OtherActor :type "Actor Object Reference") (OtherComp :type "PrimitiveComponent Object Reference") (OtherBodyIndex :type Integer) (bFromSweep :type Boolean) (SweepResult :type "HitResult Structure (by ref)"))
  (bind _returnvalue (`GameplayStatics.GetPlayerPawn` 0))
  (bind _currentconnection (`self.currentConnection`))
  (if (== OtherActor (`GameplayStatics.GetPlayerPawn` 0))
    (if (not (`self.onTeleport`))
      (set `self.isInside` true)
      (`KismetSystemLibrary.Delay` 2.0)
      (`self.closeDoors` (`self.currentConnection`))
      (`self.closeDoors`)
      (`KismetSystemLibrary.Delay` 1.0)
      (if (`self.isInside`)
        (set `/Game/Blueprints/BP_Elevator.onTeleport` true _currentconnection)
        (`KismetSystemLibrary.Delay` 1.0)
        (`self.K2_SetActorLocation` _returnvalue (+ (`SceneComponent.K2_GetComponentLocation` (`/Game/Blueprints/BP_Elevator.Base` _currentconnection)) (- (`self.K2_GetActorLocation` _returnvalue) (`SceneComponent.K2_GetComponentLocation` (`self.Base`)))) false true)
        (else
          (`self.openDoors`)))
      (else
        (`self.openDoors`)))))

(event `self.insideElevator.OnComponentEndOverlap`
  (params (OverlappedComponent :type "PrimitiveComponent Object Reference") (OtherActor :type "Actor Object Reference") (OtherComp :type "PrimitiveComponent Object Reference") (OtherBodyIndex :type Integer))
  (if (== (`GameplayStatics.GetPlayerPawn` 0) OtherActor)
    (if (`self.onTeleport`)
      (set `self.onTeleport` false))
    (set `self.isInside` false)
    (`self.closeDoors`)))

(fn `swapElevators`
  (locals (oldCurrent :type "/Game/Blueprints/BP_Elevator Object Reference"))
  (bind _output_get (set `local.oldCurrent` (`self.currentConnection`)))
  (set `self.currentConnection` (`self.otherConnection`))
  (set `self.otherConnection` _output_get))

(fn `UserConstructionScript`)