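; Level manager that runs task progression, energy countdown and channel visibility, staying inactive in the Hub and Entrance_Hub levels.
; On BeginPlay it sets the first task, shows the level title and hides "Channel" actors not tagged "1".
; renewTask advances the task, notifies "Task_N" actors through an interface and starts the timer at task 1.
; Tick then drains player energy by a frame-dependent step scaled by TimeMinutes.
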(event `self.ReceiveBeginPlay`
  (if (or (`prosperousBlueprint.IsCurrentLevel` self "/Game/Levels/Hub.Hub") (`prosperousBlueprint.IsCurrentLevel` self "/Game/Levels/Entrance_Hub.Entrance_Hub"))
    (set `self.isActive` false)
    (else
      (set `self.isActive` true)
      (`KismetSystemLibrary.Delay` 0.2)
      (`/Game/Core/PC_Player.changeTask` (cast `/Game/Core/PC_Player` (`GameplayStatics.GetPlayerController` 0) :!pure true) (`|GetArrayItem` (`self.Tasks`)))
      (`KismetSystemLibrary.Delay` 2.0)
      (`/Game/Widgets/WBP_HUD.showLevel` (cast `/Game/Widgets/WBP_HUD` (`/Game/Core/PC_Player.HUD Widget` (cast `/Game/Core/PC_Player` (`GameplayStatics.GetPlayerController` 0) :!pure true)) :!pure true) (`self.Level Title`))
      (`self.Channel Reset`))))

(event `renewTask`
  (bind _output_get (set `self.currentTask` (+ (`self.currentTask`) 1)))
  (bind _outactors (`GameplayStatics.GetAllActorsWithTag` (`KismetStringLibrary.Conv_StringToName` (`KismetStringLibrary.Concat_StrStr` "Task_" (`KismetStringLibrary.Conv_IntToString` _output_get)))))
  (for _array_element _outactors
    (if (`KismetSystemLibrary.DoesImplementInterface` _array_element "/Game/Interfaces/Int_newTaskHandler.Int_newTaskHandler_C")
      (message `/Game/Interfaces/Int_newTaskHandler.ownTaskActive` _array_element)))
  (`/Game/Core/PC_Player.changeTask` (cast `/Game/Core/PC_Player` (`GameplayStatics.GetPlayerController` 0) :!pure true) (`|GetArrayItem` (`self.Tasks`) _output_get))
  (if (== _output_get 1)
    (set `self.isTimeActivate` true)
    (set `self.startedTime` (`KismetMathLibrary.Now`))))

(event `self.ReceiveTick`
  (params (DeltaSeconds :type "Float (single-precision)"))
  (bind _playerenergy (`/Game/Core/Char_Player.playerEnergy` (cast `/Game/Core/Char_Player` (`GameplayStatics.GetPlayerPawn` 0) :!pure true)))
  (if (`self.isActive`)
    (if (`self.isTimeActivate`)
      (`KismetSystemLibrary.Delay` 0.0001)
      (bind _output_get (set `/Game/Blueprints/Player/playerEnergy.currentEnergy` (- (`/Game/Blueprints/Player/playerEnergy.currentEnergy` _playerenergy) (/ 1.0 (* (`self.Time (Minutes)`) 6000.0))) _playerenergy)))))

(event `sendChannelMessage`
  (params (setDisable :type Boolean))
  (if setDisable
    (`self.Channel Reset`)))

(fn `Channel Reset`
  (bind _outactors (`GameplayStatics.GetAllActorsWithTag` "Channel"))
  (for _array_element _outactors
    (if (not (`self.ActorHasTag` _array_element "1"))
      (`self.SetActorHiddenInGame` _array_element true)
      (`self.SetActorEnableCollision` _array_element false))))

(fn `UserConstructionScript`)