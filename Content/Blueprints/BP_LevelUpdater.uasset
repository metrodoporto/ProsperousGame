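; BP_LevelUpdater is a trigger that advances the level's task sequence when the player enters its collision.
; It finds BP_LevelCore on BeginPlay and calls RenewTask only if its TaskHandle is the next task.
; On that advance it can also start a HUD speakbox dialogue and spawn BP_EndItem at the Last actor's location.
; A separate DeletePing function, not called here, destroys nearby BP_Ping actors.
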(event `self.ReceiveBeginPlay`
  (bind _returnvalue (`GameplayStatics.GetActorOfClass` "/Game/Blueprints/BP_LevelCore.BP_LevelCore_C"))
  (set `self.LevelCore` _returnvalue))

(event `self.Collision.OnComponentBeginOverlap`
  (params (OverlappedComponent :type "PrimitiveComponent Object Reference") (OtherActor :type "Actor Object Reference") (OtherComp :type "PrimitiveComponent Object Reference") (OtherBodyIndex :type Integer) (bFromSweep :type Boolean) (SweepResult :type "HitResult Structure (by ref)"))
  (bind _levelcore (`self.LevelCore`))
  (if (== OtherActor (`GameplayStatics.GetPlayerPawn` 0))
    (if (== (+ (`/Game/Blueprints/BP_LevelCore.currentTask` _levelcore) 1) (`self.TaskHandle`))
      (`/Game/Blueprints/BP_LevelCore.renewTask` _levelcore)
      (if (`self.hasSpeakbox`)
        (`/Game/Widgets/WBP_HUD.startSpeakbox` (`/Game/Core/PC_Player.HUD (Blueprint)` (cast `/Game/Core/PC_Player` (`GameplayStatics.GetPlayerController` 0) :!pure true)) (`self.Lines`) (`self.Speaker Icon`) (`self.Speaker`)))
      (if (`self.shouldSpawnLast`)
        (`|SpawnActorFromClass` "/Game/Blueprints/Objects/BP_EndItem.BP_EndItem_C" (`KismetMathLibrary.MakeTransform` (`self.K2_GetActorLocation` (`self.Last`))) "Undefined" "MultiplyWithRoot" null null)))))

(fn `DeletePing`
  (bind _outactors (`GameplayStatics.GetAllActorsOfClass` "/Game/Blueprints/Objects/BP_Ping.BP_Ping_C"))
  (for _array_element _outactors
    (if (<= (`KismetMathLibrary.Vector_Distance` (`self.K2_GetActorLocation` _array_element) (`self.K2_GetActorLocation`)) 200.0)
      (`self.K2_DestroyActor` _array_element))))

(fn `UserConstructionScript`)