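; BP_TalkHandler runs a scripted intro dialogue in the HUD speakbox and triggers a door when it ends.
; Five seconds after BeginPlay it starts the speakbox with hardcoded Portuguese placeholder lines, a speaker name and an icon, then binds to the text's typing-finished event.
; When the last line finishes typing, a switch on an intervention counter calls ApplySecret on the Door for the first intervention and increments the counter.
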(event `self.ReceiveBeginPlay`
  (bind _array (`|MakeArray` "Dar as boas vindas e apresentar-se." "Explicar situação atual e o que se passa." "Piadola" "Abrir porta" :!type "Text"))
  (bind _aswbp_first_person_hud_a (cast `/Game/Widgets/WBP_HUD` (`/Game/Core/PC_Player.HUD Widget` (cast `/Game/Core/PC_Player` (`GameplayStatics.GetPlayerController` 0) :!pure true)) :!pure true))
  (`KismetSystemLibrary.Delay` 5.0)
  (`KismetSystemLibrary.PrintString` "Speakbox")
  (`/Game/Widgets/WBP_HUD.startSpeakbox` _aswbp_first_person_hud_a _array "/Game/Materials/2025/Images/UI_Placeholder.UI_Placeholder" "Carlos, el matador.")
  (add `sealTextWidget.OnTypingFinished` (`/Game/Widgets/WBP_SpeakBox.Text` (`/Game/Widgets/WBP_HUD.SpeakBox` _aswbp_first_person_hud_a)) (delegate `OnTypingFinished_Event`))
  (set `self.currentMax` (`KismetArrayLibrary.Array_Length` _array)))

(event `OnTypingFinished_Event`
  (if (== (+ (`/Game/Widgets/WBP_SpeakBox.currentIndex` (`/Game/Widgets/WBP_HUD.SpeakBox` (cast `/Game/Widgets/WBP_HUD` (`/Game/Core/PC_Player.HUD Widget` (cast `/Game/Core/PC_Player` (`GameplayStatics.GetPlayerController` 0) :!pure true)) :!pure true))) 1) (`self.currentMax`))
    (switch `int` (`self.Interventions`)
      (:`0`
        (`/Game/Blueprints/Objects/BP_Tutorial_Door.applySecret` (`self.Door`))
        (`/Engine/EditorBlueprintResources/StandardMacros.IncrementInt` (`self.Interventions`))))))

(fn `UserConstructionScript`)