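; BP_Water is a rising water actor that triggers a level exit when it touches the player.
; Tick runs through a short Delay, so the actor climbs in small steps at a timed rate, without sweeping.
; On overlap with the player character, it calls ExitedLevel on GI_Game with a hardcoded level name, plus the current variation and elapsed time derived from BP_LevelCore.
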(event `self.ReceiveActorBeginOverlap`
  (params (OtherActor :type "Actor Object Reference"))
  (if (== OtherActor (`GameplayStatics.GetPlayerCharacter` 0))
    (bind _returnvalue (`GameplayStatics.GetActorOfClass` "/Game/Blueprints/BP_LevelCore.BP_LevelCore_C"))
    (`/Game/Core/GI_Game.exitedLevel` (cast `/Game/Core/GI_Game` (`GameplayStatics.GetGameInstance`) :!pure true) false "news" (`/Game/Blueprints/BP_LevelCore.CurrentVariation` _returnvalue) (- (`KismetMathLibrary.Now`) (`/Game/Blueprints/BP_LevelCore.startedTime` _returnvalue)))))

(event `self.ReceiveTick`
  (params (DeltaSeconds :type "Float (single-precision)"))
  (`KismetSystemLibrary.Delay` 0.05)
  (`self.K2_SetActorLocation` (+ (`self.K2_GetActorLocation`) (0.0 0.0 1.0))))

(fn `UserConstructionScript`)