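; BP_levelFinisher is a level goal trigger that ends the level as a win and returns the player to the hub.
; On BeginPlay it caches the BP_LevelCore actor found in the world.
; When the player pawn overlaps its Collision component, it calls ChangeToHub on GI_Game with a "Won!" reason.
; It passes the elapsed time since the core's StartedTime as the RemainingTime argument.
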(event `self.ReceiveBeginPlay`
  (bind _returnvalue (`GameplayStatics.GetActorOfClass` "/Game/Blueprints/BP_LevelCore.BP_LevelCore_C"))
  (set `self.LevelCore` _returnvalue))

(event `self.Collision.OnComponentBeginOverlap`
  (params (OverlappedComponent :type "PrimitiveComponent Object Reference") (OtherActor :type "Actor Object Reference") (OtherComp :type "PrimitiveComponent Object Reference") (OtherBodyIndex :type Integer) (bFromSweep :type Boolean) (SweepResult :type "HitResult Structure (by ref)"))
  (if (== OtherActor (`GameplayStatics.GetPlayerPawn` 0))
    (`/Game/Core/GI_Game.changeToHub` (cast `/Game/Core/GI_Game` (`GameplayStatics.GetGameInstance`) :!pure true) (- (`KismetMathLibrary.Now`) (`/Game/Blueprints/BP_LevelCore.startedTime` (`self.LevelCore`))) "Won!")))

(fn `UserConstructionScript`)