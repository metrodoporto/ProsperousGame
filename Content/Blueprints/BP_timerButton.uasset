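; BP_timerButton is an interactable button that starts a timer on a referenced Clock.
; On interact, it calls StartTimer on the Clock only if that timer is not already running.
; OpenDoor is an empty event, and the elevator swap, door-opening and timeline-driven vertical movement chains are disconnected leftovers that never run.
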(event `self.ReceiveBeginPlay`)

(event `OpenDoor`)

(event `self.onInteract`
  (params (Component :type "PrimitiveComponent Object Reference"))
  (bind _clock (`self.Clock`))
  (if (not (`/Game/Blueprints/Objects/BP_clockTimer.onTimer` _clock))
    (`/Game/Blueprints/Objects/BP_clockTimer.startTimer` _clock)))

(fn `UserConstructionScript`)