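; LevelUpdater is an actor that advances the level's task progression when the player reaches it.
; On BeginPlay it finds and stores the LevelCore actor in the level.
; When the player pawn overlaps its Collision component and its TaskHandle is the next task after LevelCore's CurrentTask, it calls RenewTask on LevelCore, so triggers only fire in sequence.
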(event `self.ReceiveBeginPlay`
  (bind _returnvalue (`GameplayStatics.GetActorOfClass` "/Game/Blueprints/LevelCore.LevelCore_C"))
  (set `self.LevelCore` _returnvalue))

(event `self.Collision.OnComponentBeginOverlap`
  (params (OverlappedComponent :type "PrimitiveComponent Object Reference") (OtherActor :type "Actor Object Reference") (OtherComp :type "PrimitiveComponent Object Reference") (OtherBodyIndex :type Integer) (bFromSweep :type Boolean) (SweepResult :type "HitResult Structure (by ref)"))
  (bind _levelcore (`self.LevelCore`))
  (if (== OtherActor (`GameplayStatics.GetPlayerPawn` 0))
    (if (== (+ (`/Game/Blueprints/LevelCore.currentTask` _levelcore) 1) (`self.TaskHandle`))
      (`/Game/Blueprints/LevelCore.renewTask` _levelcore))))

(fn `UserConstructionScript`)