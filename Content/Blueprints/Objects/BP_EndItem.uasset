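; BP_EndItem is the level's interactable goal object, with mesh, materials, rotation and scale applied in the construction script.
; Interacting either opens a WBP_FloatScreen confirmation or records the completed level and reports the win with elapsed time to GI_Game, using BP_LevelCore data.
; Tick spins the widget in Delay-throttled steps.
; For the LowpolyCD mesh only, a timeline floats and rotates it while Tick turns the actor and spring arm toward the player.
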(event `Animation`
  (bind _widget (`self.Widget`))
  (bind (_relativerotation_roll _relativerotation_pitch _relativerotation_yaw) (`KismetMathLibrary.BreakRotator` (`SceneComponent.RelativeRotation` _widget)))
  (`KismetSystemLibrary.Delay` 0.05)
  (`SceneComponent.K2_SetRelativeRotation` _widget (`KismetMathLibrary.MakeRotator` (+ _relativerotation_roll 5.0) _relativerotation_pitch _relativerotation_yaw) false false))

(event `self.ReceiveTick`
  (params (DeltaSeconds :type "Float (single-precision)"))
  (bind (_returnvalue_roll _returnvalue_pitch) (`KismetMathLibrary.BreakRotator` (`self.K2_GetActorRotation`)))
  (bind (_returnvalue_roll_2 _returnvalue_pitch_2 _returnvalue_yaw) (`KismetMathLibrary.BreakRotator` (`KismetMathLibrary.FindLookAtRotation` (`self.K2_GetActorLocation`) (`self.K2_GetActorLocation` (`GameplayStatics.GetPlayerCharacter` 0)))))
  (`self.Animation`)
  (if (== (`self.Mesh`) "/Game/Models/GeneralUse/CD/LowpolyCD.LowpolyCD")
    (`self.K2_SetActorRotation` (`KismetMathLibrary.MakeRotator` _returnvalue_roll _returnvalue_pitch (+ _returnvalue_yaw -90.0)))
    (`SceneComponent.K2_SetRelativeRotation` (`self.SpringArm`) (`KismetMathLibrary.MakeRotator` _returnvalue_roll_2 _returnvalue_pitch_2 90.0) false false)))

(event `/Game/Interfaces/Int_Interactable.onInteract`
  (bind _returnvalue (`GameplayStatics.GetPlayerController` 0))
  (bind _asgi_game (cast `/Game/Core/GI_Game` (`GameplayStatics.GetGameInstance`) :!pure true))
  (if (`self.askConfirmation`)
    (bind _returnvalue_2 (`|CreateWidget` "/Game/Widgets/WBP_FloatScreen.WBP_FloatScreen_C" null 3))
    (`UserWidget.AddToViewport` _returnvalue_2 999)
    (`WidgetBlueprintLibrary.SetInputMode_UIOnlyEx` _returnvalue null)
    (set `PlayerController.bShowMouseCursor` true _returnvalue)
    (else
      (bind _returnvalue_3 (`GameplayStatics.GetActorOfClass` "/Game/Blueprints/BP_LevelCore.BP_LevelCore_C"))
      (`KismetSystemLibrary.PrintString` "Won")
      (bind _name (`/Game/Blueprints/BP_LevelCore.Name` _returnvalue_3))
      (bind _currentvariation (`/Game/Blueprints/BP_LevelCore.CurrentVariation` _returnvalue_3))
      (`/Game/Core/GI_Game.addCompletedLevel` _asgi_game (make `/Game/Structures/ST_playerLevel` _name _currentvariation))
      (`/Game/Core/GI_Game.exitedLevel` _asgi_game true _name _currentvariation (- (`KismetMathLibrary.Now`) (`/Game/Blueprints/BP_LevelCore.startedTime` _returnvalue_3))))))

(event `self.ReceiveBeginPlay`
  (bind _level (`self.Level`))
  (if (== (`self.Mesh`) "/Game/Models/GeneralUse/CD/LowpolyCD.LowpolyCD")
    (bind (_direction _floatpos _rotation) (`Timeline|loop` :!via `PlayFromStart`)
      (:`Update`
        (`SceneComponent.K2_AddLocalOffset` _level (`KismetMathLibrary.MakeVector` 0.0 0.0 (* _floatpos 0.3)) false false)
        (`SceneComponent.K2_AddLocalRotation` _level (`KismetMathLibrary.MakeRotator` 0.0 (* _rotation 0.2) (* _rotation 0.3)) false false)))))

(fn `UserConstructionScript`
  (bind _level (`self.Level`))
  (`StaticMeshComponent.SetStaticMesh` _level (`self.Mesh`))
  (for (_array_element _array_index) (`self.Material`)
    (`PrimitiveComponent.SetMaterial` _level _array_index _array_element))
  (`SceneComponent.K2_SetRelativeRotation` _level (`self.Rotation`) false false)
  (`SceneComponent.SetRelativeScale3D` _level (`self.Scale`)))