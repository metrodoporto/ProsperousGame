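; BP_LevelSelector is an interactable level selector object with left and right arrow components and a level component.
; OnInteract checks which component was used, routing the right or left arrow parts to ChangeRight or ChangeLeft and opening the DevMovement level from the Level component.
; Selection is a stub: both change events only print their direction, SetView is empty, and the target level is fixed.
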(event `self.onInteract`
  (params (Component :type "PrimitiveComponent Object Reference"))
  (if (or (== Component (`self.RArrow`)) (== Component (`self.arrow2`)) (== Component (`self.arrow1`)))
    (`self.ChangeRight`)
    (elif (or (== Component (`self.LArrow`)) (== Component (`self.arrow4`)) (== Component (`self.arrow3`)))
      (`self.ChangeLeft`)
      (elif (== Component (`self.Level`))
        (`GameplayStatics.OpenLevelBySoftObjectPtr` "/Game/Levels/DevRooms/devMovement.devMovement")))))

(event `self.setView`
  (params (isViewing :type Boolean)))

(event `ChangeRight`
  (`KismetSystemLibrary.PrintString` "Right"))

(event `ChangeLeft`
  (`KismetSystemLibrary.PrintString` "Left"))

(fn `UserConstructionScript`)