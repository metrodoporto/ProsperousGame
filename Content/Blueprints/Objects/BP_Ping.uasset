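; BP_Ping is a world ping marker that shows colored text and the player's distance to it through an InGameUI_Ping widget.
; On BeginPlay it casts its widget component to InGameUI_Ping, passes in its Color and Text, and caches the DistanceText block.
; Every Tick it sets that block to the distance from the player pawn, converted to whole meters with an "m" suffix.
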(event `self.ReceiveBeginPlay`
  (bind _asin_game_ui_ping (cast `/Game/Widgets/GeneralUse/InGameUI_Ping` (`WidgetComponent.GetWidget` (`self.Widget`))))
  (set `/Game/Widgets/GeneralUse/InGameUI_Ping.Color` (`self.Color`) _asin_game_ui_ping)
  (set `/Game/Widgets/GeneralUse/InGameUI_Ping.Text` (`self.Text`) _asin_game_ui_ping)
  (set `self.Distance Text` (`/Game/Widgets/GeneralUse/InGameUI_Ping.DistanceText` _asin_game_ui_ping)))

(event `self.ReceiveTick`
  (params (DeltaSeconds :type "Float (single-precision)"))
  (`TextBlock.SetText` (`self.Distance Text`) (`KismetTextLibrary.Conv_StringToText` (`KismetStringLibrary.Concat_StrStr` (`KismetStringLibrary.Conv_IntToString` (`KismetMathLibrary.FTrunc` (/ (`KismetMathLibrary.Vector_Distance` (`self.K2_GetActorLocation`) (`self.K2_GetActorLocation` (`GameplayStatics.GetPlayerPawn` 0))) 100.0))) "m"))))

(fn `UserConstructionScript`)