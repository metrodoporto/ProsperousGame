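; BP_PuzzleGate is a double-door gate that opens once enough items have been collected.
; CollectItem increments the count, and both it and OnInteract check it against the required maximum.
; The first successful check, guarded by DoOnce, starts a timeline that swings both door sides, calls RenewTask on BP_LevelCore and spawns a CD-mesh BP_EndItem at ItemSpawn.
; When the swing finishes, a colored BP_Ping spawns above the gate.
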(event `Open Door`
  (bind (_direction _door_rotation) (`Timeline|Open Door Anim` :!via `PlayFromStart`)
    (:`Update`
      (`SceneComponent.K2_SetRelativeRotation` (`self.DoorSide1`) (`KismetMathLibrary.MakeRotator` 0.0 0.0 (`KismetMathLibrary.Lerp` 90.0 175.0 _door_rotation)) false false)
      (`SceneComponent.K2_SetRelativeRotation` (`self.DoorSide`) (`KismetMathLibrary.MakeRotator` 0.0 0.0 (`KismetMathLibrary.Lerp` 90.0 5.0 _door_rotation)) false false))
    (:`Finished`
      (`|SpawnActorFromClass` "/Game/Blueprints/Objects/BP_Ping.BP_Ping_C" (`KismetMathLibrary.Conv_VectorToTransform` (+ (`self.K2_GetActorLocation`) (0.0 0.0 100.0))) "Undefined" "MultiplyWithRoot" null (struct :`R` 0.379385 :`B` 1.0 :`A` 1.0) null))))

(event `Collect Item`
  (`/Engine/EditorBlueprintResources/StandardMacros.IncrementInt` (`self.currentItemsCollected`)
    (:`  `
      (`self.Open Door Check` :!label _label))))

(event `/Game/Interfaces/Int_Interactable.onInteract`
  (goto _label))

(event `Open Door Check`
  (if (>= (`self.currentItemsCollected`) (`self.maxItemsCollected`))
    (`/Engine/EditorBlueprintResources/StandardMacros.DoOnce` false
      (:`Completed`
        (`self.Open Door`)
        (bind _returnvalue (`GameplayStatics.GetActorOfClass` "/Game/Blueprints/BP_LevelCore.BP_LevelCore_C"))
        (`/Game/Blueprints/BP_LevelCore.renewTask` _returnvalue)
        (`|SpawnActorFromClass` "/Game/Blueprints/Objects/BP_EndItem.BP_EndItem_C" (`KismetMathLibrary.MakeTransform` (`self.K2_GetActorLocation` (`self.ItemSpawn`))) "Undefined" "MultiplyWithRoot" null "/Game/Models/GeneralUse/CD/LowpolyCD.LowpolyCD" (`|MakeArray` "/Game/Models/GeneralUse/CD/CD_Mat.CD_Mat" :!type "MaterialInterface Object Reference") (struct :`Roll` -10.0) (0.06 0.06 0.06) false null)))))

(fn `UserConstructionScript`)