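; Puzzle table that displays collection progress from the BP_PuzzleGate and can open two doors.
; Construction script shows either the cult or const table mesh based on IsNews.
; Each Tick updates the widget's collected/max text and, when IsNews is off, reveals up to four cassettes to match the count.
; It also triggers both doors' Goto whenever the NAND of completion and IsNews is true.
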(event `openTheGates`
  (`/Game/Models/Crane/BP_Crane.goto` (`self.Door1`) -35.0 2300.0 2750.0 90.0)
  (`/Game/Models/Crane/BP_Crane.goto` (`self.Door2`) -147.0 3600.0 3400.0 220.0))

(event `self.ReceiveTick`
  (params (DeltaSeconds :type "Float (single-precision)"))
  (`self.updateText`))

(event `updateText`
  (bind _returnvalue (`GameplayStatics.GetActorOfClass` "/Game/Blueprints/Objects/BP_PuzzleGate.BP_PuzzleGate_C"))
  (bind _currentitemscollected (`/Game/Blueprints/Objects/BP_PuzzleGate.currentItemsCollected` _returnvalue))
  (bind _maxitemscollected (`/Game/Blueprints/Objects/BP_PuzzleGate.maxItemsCollected` _returnvalue))
  (set `/Game/Widgets/UW_Text.Text` (`|FormatText` "{0} / {1}" _currentitemscollected _maxitemscollected) (cast `/Game/Widgets/UW_Text` (`WidgetComponent.GetWidget` (`self.Widget`)) :!pure true))
  (`self.updateVisible` _currentitemscollected)
  (if (`KismetMathLibrary.BooleanNAND` (== _currentitemscollected _maxitemscollected) (`self.isNews`))
    (`self.openTheGates`)))

(event `updateVisible`
  (params (Current :type Integer))
  (if (not (`self.isNews`))
    (bind _output_get (set `self.tempCur` Current))
    (if (> _output_get 0)
      (`SceneComponent.SetVisibility` (`self.Cassette`) true false)
      (bind _result (`/Engine/EditorBlueprintResources/StandardMacros.DecrementInt` _output_get)
        (:`  `
          (if (> _result 0)
            (`SceneComponent.SetVisibility` (`self.Cassette1`) true false)
            (bind _result_2 (`/Engine/EditorBlueprintResources/StandardMacros.DecrementInt` _result)
              (:`  `
                (if (> _result_2 0)
                  (`SceneComponent.SetVisibility` (`self.Cassette2`) true false)
                  (bind _result_3 (`/Engine/EditorBlueprintResources/StandardMacros.DecrementInt` _result_2)
                    (:`  `
                      (if (> _result_3 0)
                        (`SceneComponent.SetVisibility` (`self.Cassette3`) true false)))))))))))))

(fn `UserConstructionScript`
  (bind _isnews (`self.isNews`))
  (`SceneComponent.SetVisibility` (`self.CultTable`) (not _isnews) true)
  (`SceneComponent.SetVisibility` (`self.ConstTable`) _isnews true))