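; BP_Tutorial_Door is a tutorial door that slides open when its applySecret event is triggered.
; The event plays the DoorScale timeline from the start, moving two mirrored pairs of components apart along local Y.
; The SmallDoor track drives Cube and Cube1, while the BigDoor track drives TutDoor and TutDoor1.
; A delayed debug print and self-call to ApplySecret remain in the graph, disconnected.
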(event `self.ReceiveBeginPlay`)

(event `applySecret`
  (bind (_direction _bigdoor _smalldoor) (`Timeline|DoorScale` :!via `PlayFromStart`)
    (:`Update`
      (`SceneComponent.K2_SetRelativeLocation` (`self.Cube`) (`KismetMathLibrary.MakeVector` 0.0 (+ (* _smalldoor -200.0) -200.0) 300.0) false false)
      (`SceneComponent.K2_SetRelativeLocation` (`self.Cube1`) (`KismetMathLibrary.MakeVector` 0.0 (+ (* _smalldoor 200.0) 200.0) 300.0) false false)
      (bind _returnvalue (* _bigdoor 190.0))
      (`SceneComponent.K2_SetRelativeLocation` (`self.tutDoor`) (`KismetMathLibrary.MakeVector` 0.0 (+ _returnvalue 402.5)) false false)
      (`SceneComponent.K2_SetRelativeLocation` (`self.tutDoor1`) (`KismetMathLibrary.MakeVector` 0.0 (+ (* _returnvalue -1.0) -402.5)) false false))))

(fn `UserConstructionScript`)