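; BP_channelObject is a configurable mesh object that can be switched between visible and hidden.
; The construction script applies the mesh, material and separate scales for the Model and Collision components from its variables.
; The switchMe event sets Model visibility without propagating to children and toggles its collision between query-and-physics and none, leaving the Collision component untouched.
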(event `switchMe`
  (params (toVisible :type Boolean))
  (bind _model (`self.Model`))
  (`SceneComponent.SetVisibility` _model toVisible false)
  (`PrimitiveComponent.SetCollisionEnabled` _model (select `bool` toVisible :`false` "NoCollision" :`true` "QueryAndPhysics" :!type "ECollisionEnabled Enum")))

(fn `UserConstructionScript`
  (bind _model (`self.Model`))
  (`SceneComponent.SetRelativeScale3D` (`self.Collision`) (`self.Collision Scale`))
  (`SceneComponent.SetRelativeScale3D` _model (`self.Model Scale`))
  (`StaticMeshComponent.SetStaticMesh` _model (`self.Mesh`))
  (`PrimitiveComponent.SetMaterial` _model 0 (`self.Material`)))