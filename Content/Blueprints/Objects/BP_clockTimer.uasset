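; Clock timer actor that shows a millisecond readout on a text render and can open a referenced BigDoor.
; startTimer flags OnTimer and plays a timeline whose track drives the text, unless the timer is already finished.
; openDoor opens the door and sets IsFinished.
; When the timeline ends, OnTimer clears and the text shows OPEN if finished, otherwise resets to its default time.
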(event `startTimer`
  (bind _textrender (`self.TextRender`))
  (if (not (`self.isFinished`))
    (set `self.onTimer` true)
    (bind (_direction _newtrack_0) (`Timeline|Timer` :!via `PlayFromStart`)
      (:`Update`
        (`TextRenderComponent.K2_SetText` (`self.TextRender`) (`|FormatText` "{0}ms" (`KismetTextLibrary.Conv_DoubleToText` _newtrack_0 "HalfToEven" false true 1 1 3))))
      (:`Finished`
        (set `self.onTimer` false)
        (if (`self.isFinished`)
          (`TextRenderComponent.K2_SetText` _textrender "OPEN")
          (else
            (`TextRenderComponent.K2_SetText` _textrender "4,000ms")))))))

(event `openDoor`
  (`/Game/Blueprints/Objects/BP_bigDoor.openDoor` (`self.bigDoor`))
  (set `self.isFinished` true))

(fn `UserConstructionScript`)