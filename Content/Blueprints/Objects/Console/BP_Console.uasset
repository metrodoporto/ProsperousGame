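; BP_Console is an interactable in-world console with a widget screen the player can use.
; On interact, it blends the camera to itself, turns on widget hit testing and the mouse cursor, and switches input to UI-only.
; LeaveConsole reverses this, returning the view to the stored player character.
; It passes itself to its Console_Layout widget, and SetView switches that layout between two screens.
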(event `self.ReceiveBeginPlay`
  (set `/Game/Widgets/Console/Console_Layout.Console` self (cast `/Game/Widgets/Console/Console_Layout` (`WidgetComponent.GetWidget` (`self.Widget`)) :!pure true)))

(event `LeaveConsole`
  (bind _returnvalue (`GameplayStatics.GetPlayerController` 0))
  (`PlayerController.SetViewTargetWithBlend` _returnvalue (stale `/Game/Interfaces/Int_Interactable.onInteract` _output_get) 0.2 "VTBlend_EaseIn" 1.0 false)
  (set `WidgetInteractionComponent.bEnableHitTesting` false (`self.WidgetInteraction`))
  (set `PlayerController.bShowMouseCursor` false _returnvalue)
  (`WidgetBlueprintLibrary.SetInputMode_GameOnly` _returnvalue))

(event `/Game/Interfaces/Int_Interactable.onInteract`
  (bind _returnvalue (`GameplayStatics.GetPlayerController` 0))
  (bind _output_get (set `self.PlayerCam` (cast `/Game/Core/Char_Player` (`GameplayStatics.GetPlayerCharacter` 0) :!pure true)))
  (`PlayerController.SetViewTargetWithBlend` _returnvalue self 0.2 "VTBlend_EaseIn" 1.0 false)
  (set `WidgetInteractionComponent.bEnableHitTesting` true (`self.WidgetInteraction`))
  (set `PlayerController.bShowMouseCursor` true _returnvalue)
  (`WidgetBlueprintLibrary.SetInputMode_UIOnlyEx` _returnvalue null))

(event `/Game/Interfaces/Int_Interactable.setView`
  (params (isViewing :type Boolean))
  (bind _asconsole_layout (cast `/Game/Widgets/Console/Console_Layout` (`WidgetComponent.GetWidget` (`self.Widget`)) :!pure true))
  (if isViewing
    (`/Game/Widgets/Console/Console_Layout.ChangeScreen` _asconsole_layout 1)
    (else
      (`/Game/Widgets/Console/Console_Layout.ChangeScreen` _asconsole_layout 0))))

(fn `UserConstructionScript`)