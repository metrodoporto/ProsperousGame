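; OilPuddle_BP is an oil puddle hazard that hinders the player while they stand in it.
; When a Char_Player overlaps its Box, it cuts the character's max walk speed and jump velocity to fractions of the player's stored defaults.
; Leaving the Box restores both values from those same defaults on the character's movement component.
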(event `self.Box.OnComponentBeginOverlap`
  (params (OverlappedComponent :type "PrimitiveComponent Object Reference") (OtherActor :type "Actor Object Reference") (OtherComp :type "PrimitiveComponent Object Reference") (OtherBodyIndex :type Integer) (bFromSweep :type Boolean) (SweepResult :type "HitResult Structure (by ref)"))
  (bind _aschar_player (cast `/Game/Core/Char_Player` OtherActor))
  (bind _charactermovement (`Character.CharacterMovement` _aschar_player))
  (set `CharacterMovementComponent.MaxWalkSpeed` (* (`/Game/Core/Char_Player.DefaultMaxSpeed` _aschar_player) 0.25) _charactermovement)
  (set `CharacterMovementComponent.JumpZVelocity` (* (`/Game/Core/Char_Player.DefaultJumpZ` _aschar_player) 0.3) _charactermovement))

(event `self.Box.OnComponentEndOverlap`
  (params (OverlappedComponent :type "PrimitiveComponent Object Reference") (OtherActor :type "Actor Object Reference") (OtherComp :type "PrimitiveComponent Object Reference") (OtherBodyIndex :type Integer))
  (bind _aschar_player (cast `/Game/Core/Char_Player` OtherActor))
  (bind _charactermovement (`Character.CharacterMovement` _aschar_player))
  (set `CharacterMovementComponent.MaxWalkSpeed` (`/Game/Core/Char_Player.DefaultMaxSpeed` _aschar_player) _charactermovement)
  (set `CharacterMovementComponent.JumpZVelocity` (`/Game/Core/Char_Player.DefaultJumpZ` _aschar_player) _charactermovement))

(fn `UserConstructionScript`)