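; devIntBlock is a developer test interactable that instantly completes a level when used.
; On interact it prints a win message, records a "debug" level as completed in GI_Game, then calls ExitedLevel as true.
; A view event prints debug text as the block gains or loses the viewer's focus.
; Unconnected leftover nodes hold startup widget creation and a profile-update, delayed-exit test.
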(event `/Game/Interfaces/Int_Interactable.onInteract`
  (params (Component :type "PrimitiveComponent Object Reference"))
  (bind _asgi_game (cast `/Game/Core/GI_Game` (`GameplayStatics.GetGameInstance`) :!pure true))
  (`KismetSystemLibrary.PrintString` "Won")
  (`/Game/Core/GI_Game.addCompletedLevel` _asgi_game (make `/Game/Structures/ST_playerLevel` "debug" 1))
  (`/Game/Core/GI_Game.exitedLevel` _asgi_game true))

(event `setView_1`
  (params (isViewing :type Boolean))
  (if isViewing
    (`KismetSystemLibrary.PrintString` "dev YA")
    (else
      (`KismetSystemLibrary.PrintString` "dev NAY"))))

(fn `UserConstructionScript`)