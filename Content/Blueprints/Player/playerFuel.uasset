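; Player fuel Blueprint that tracks a spendable fuel pool with delayed regeneration.
; UseFuel deducts the requested amount and restarts a short cooldown if enough fuel remains, returning whether it succeeded.
; Tick counts the cooldown down in one-second steps, then adds fuel in small increments until the maximum is reached.
; Both timings rely on Delay nodes on Tick, so the refill rate can vary with frame rate.
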(event `self.ReceiveTick`
  (params (DeltaSeconds :type "Float (single-precision)"))
  (if (> (`self.inCooldown`) 0)
    (`KismetSystemLibrary.Delay` 1.0)
    (set `self.inCooldown` (- (`self.inCooldown`) 1))
    (elif (not (>= (`self.currentFuel`) (`self.maxFuel`)))
      (`KismetSystemLibrary.Delay` 0.005)
      (set `self.currentFuel` (+ (`self.currentFuel`) 0.007)))))

(fn `Use Fuel`
  (params (`Used Fuel` :type "Float (double-precision)"))
  (returns (Executed :type Boolean))
  (if (<= `Used Fuel` (`self.currentFuel`))
    (set `self.currentFuel` (- (`self.currentFuel`) `Used Fuel`))
    (set `self.inCooldown` 3)
    (return true)
    (else
      (return false))))