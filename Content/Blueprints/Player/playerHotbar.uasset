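; Player hotbar Blueprint that tracks owned ability modules and their assignment to hotbar slots.
; On BeginPlay it sizes the slot array, and functions set, clear or look up a module's slot, with lookup returning -1 when absent.
; Unlocking adds a module ID to the inventory, which the ownership check searches.
; SetHotbar runs that check but writes the slot regardless of the result.
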(event `self.ReceiveBeginPlay`
  (`KismetArrayLibrary.Array_Resize` (`self.hotbarSlots`) (`self.hotbarSize`)))

(fn `checkModule`
  (params (`Module ID` :type String))
  (returns (Slot :type Integer))
  (for (_array_element _array_index) (`self.hotbarSlots`)
    (if (`KismetStringLibrary.EqualEqual_StrStr` _array_element `Module ID`)
      (return _array_index)))
  (return -1))

(fn `clearSlot`
  (params (Slot :type Integer))
  (`KismetArrayLibrary.Array_Set` (`self.hotbarSlots`) Slot))

(fn `setHotbar`
  (params (moduleID :type String) (slot :type Integer))
  (bind _hasownership (`self.validateOwnership` moduleID))
  (if _hasownership
    _
    (else
      _))
  (`KismetArrayLibrary.Array_Set` (`self.hotbarSlots`) slot moduleID))

(fn `unlockAbility`
  (params (`Module ID` :type String))
  (`KismetArrayLibrary.Array_Add` (`self.Inventory`) `Module ID`))

(fn `validateOwnership`
  (params (`Module ID` :type String))
  (returns (hasOwnership :type Boolean))
  (return (!= (`KismetArrayLibrary.Array_Find` (`self.Inventory`) `Module ID`) -1)))