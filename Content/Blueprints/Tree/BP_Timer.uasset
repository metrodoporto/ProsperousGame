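; BP_Timer is a box trigger that either starts or finishes a timed run when the player pawn overlaps it.
; On overlap it looks up the BP_TimerCore actor and branches on the IsStart flag.
; A start trigger activates the timer and destroys itself.
; Otherwise it calls ChangeToHub on GI_Game, passing the timer's time as remaining time with a win reason.
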(event `self.ReceiveBeginPlay`)

(event `self.Box.OnComponentBeginOverlap`
  (params (OverlappedComponent :type "PrimitiveComponent Object Reference") (OtherActor :type "Actor Object Reference") (OtherComp :type "PrimitiveComponent Object Reference") (OtherBodyIndex :type Integer) (bFromSweep :type Boolean) (SweepResult :type "HitResult Structure (by ref)"))
  (if (== OtherActor (`GameplayStatics.GetPlayerPawn` 0))
    (bind _returnvalue (`GameplayStatics.GetActorOfClass` "/Game/Blueprints/Tree/BP_TimerCore.BP_TimerCore_C"))
    (if (`self.isStart`)
      (`/Game/Blueprints/Tree/BP_TimerCore.activateTimer` _returnvalue)
      (`self.K2_DestroyActor`)
      (else
        (`/Game/Core/GI_Game.changeToHub` (cast `/Game/Core/GI_Game` (`GameplayStatics.GetGameInstance`) :!pure true) (`/Game/Blueprints/Tree/BP_TimerCore.Time` _returnvalue) "Won!")))))

(fn `UserConstructionScript`)