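; Countdown timer core that builds a duration from Minutes and tracks remaining time against a wall-clock goal.
; Tick updates Timer from GoalTime minus Now while HasStarted, then calls TimeFinishes, which prints a debug string and stops it.
; AddTimer extends the goal, FinishTimer stops the countdown, and ActivateTimer is an empty event.
; The start logic, time-out return to the hub and time readout are disconnected, so nothing here starts the countdown.
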(event `self.ReceiveBeginPlay`
  (set `self.Time` (`KismetMathLibrary.MakeTimespan` 0 0 (`self.Minutes`))))

(event `self.ReceiveTick`
  (params (DeltaSeconds :type "Float (single-precision)"))
  (bind _returnvalue (- (`self.goalTime`) (`KismetMathLibrary.Now`)))
  (if (`self.hasStarted`)
    (if (<= (`KismetMathLibrary.MakeTimespan` 0) _returnvalue)
      (bind _output_get (set `self.Timer` _returnvalue))
      (else
        (`self.timeFinishes`)))))

(event `activateTimer`)

(event `addTimer`
  (params (Seconds :type Integer))
  (set `self.goalTime` (+ (`self.goalTime`) (`KismetMathLibrary.MakeTimespan` 0 0 0 Seconds))))

(event `timeFinishes`
  (`KismetSystemLibrary.PrintString` "Hello")
  (set `self.hasStarted` false))

(event `finishTimer`
  (set `self.hasStarted` false))

(fn `UserConstructionScript`)