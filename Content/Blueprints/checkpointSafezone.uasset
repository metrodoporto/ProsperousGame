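; Checkpoint safezone actor that pauses the level timer while the player stands inside its box volume.
; Box overlap begin and end events filter for player pawn 0, then look up the LevelCore actor with GetActorOfClass.
; If that LevelCore has a timer, entering sets IsTimeActivate false and leaving sets it back to true.
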(event `self.Box.OnComponentBeginOverlap`
  (params (OverlappedComponent :type "PrimitiveComponent Object Reference") (OtherActor :type "Actor Object Reference") (OtherComp :type "PrimitiveComponent Object Reference") (OtherBodyIndex :type Integer) (bFromSweep :type Boolean) (SweepResult :type "HitResult Structure (by ref)"))
  (if (== OtherActor (`GameplayStatics.GetPlayerPawn` 0))
    (bind _returnvalue (`GameplayStatics.GetActorOfClass` "/Game/Blueprints/LevelCore.LevelCore_C"))
    (if (`/Game/Blueprints/LevelCore.hasTimer` _returnvalue)
      (set `/Game/Blueprints/LevelCore.isTimeActivate` false _returnvalue))))

(event `self.Box.OnComponentEndOverlap`
  (params (OverlappedComponent :type "PrimitiveComponent Object Reference") (OtherActor :type "Actor Object Reference") (OtherComp :type "PrimitiveComponent Object Reference") (OtherBodyIndex :type Integer))
  (if (== OtherActor (`GameplayStatics.GetPlayerPawn` 0))
    (bind _returnvalue (`GameplayStatics.GetActorOfClass` "/Game/Blueprints/LevelCore.LevelCore_C"))
    (if (`/Game/Blueprints/LevelCore.hasTimer` _returnvalue)
      (set `/Game/Blueprints/LevelCore.isTimeActivate` true _returnvalue))))

(fn `UserConstructionScript`)