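; Player controller that creates the HUD, registers input and drives two world-altering abilities through actor tags.
; Q swaps between two channels, toggling visibility and collision on "Channel" actors.
; Tab temporarily reveals and solidifies hidden "RGB" actors while overriding the pawn camera's post-process, with a flag blocking re-triggering until it reverts.
; Holding Escape shows a quit overlay and exits the game after a timed hold.
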(event `hideHUD`
  (`/Game/Widgets/UW_HUD.HideSelf` (`self.HUD`)))

(event `showHUD`
  (`UserWidget.AddToViewport` (`self.HUD`) -1))

(event `self.ReceiveBeginPlay`
  (bind _returnvalue (== (`self.activeChannel`) 1))
  (bind _returnvalue_2 (not _returnvalue))
  ;[1 0 0.2109] BeginPlay Event
  (`self.setUp`)
  (`|ExecutionSequence`
    (:`then_0`
      (bind _outactors (`GameplayStatics.GetAllActorsWithTag` "Channel"))
      (for _array_element _outactors
        (if (`self.ActorHasTag` _array_element "1")
          (`self.SetActorHiddenInGame` _array_element _returnvalue_2)
          (`self.SetActorEnableCollision` _array_element _returnvalue)
          (else
            (`self.SetActorHiddenInGame` _array_element _returnvalue)
            (`self.SetActorEnableCollision` _array_element _returnvalue_2)))))
    (:`then_1`
      (bind _outactors_2 (`GameplayStatics.GetAllActorsWithTag` "RGB"))
      (for _array_element_2 _outactors_2
        (`self.SetActorHiddenInGame` _array_element_2 true)
        (`self.SetActorEnableCollision` _array_element_2 false)))))

(event `EnhancedInput|/Game/Core/Inputs/IA_Escape`
  (params (ActionValue :type Boolean) (ElapsedSeconds :type "Float (double-precision)") (TriggeredSeconds :type "Float (double-precision)") (InputAction :type "InputAction Object Reference" :default "/Game/Core/Inputs/IA_Escape.IA_Escape"))
  (:`Triggered`
    (if (>= ElapsedSeconds 5.0) :!label _label
      (`KismetSystemLibrary.QuitGame` null "Quit")))
  (:`Started`
    (bind _returnvalue (`|CreateWidget` "/Game/Widgets/UWidget_Overlay_Quit.UWidget_Overlay_Quit_C"))
    (bind _output_get (set `self.QuitOverlay` _returnvalue))
    (`UserWidget.AddToViewport` _returnvalue 0)
    (`UserWidget.AddToViewport` _output_get 0))
  (:`Canceled`
    (`Widget.RemoveFromParent` (`self.QuitOverlay`)))
  (:`Completed`
    (goto _label)))

(event `Key|Q`
  (params (Key :type "Key Structure"))
  (:`Pressed`
    (`self.swapChannel`)
    (`KismetSystemLibrary.PrintString` "channel Swap!")))

(event `swapChannel`
  (bind _returnvalue (== (`self.activeChannel`) 1))
  (bind _returnvalue_2 (not _returnvalue))
  ;[1 1 1] Swap Channel Ability
  (bind _outactors (`GameplayStatics.GetAllActorsWithTag` "Channel"))
  (for _array_element _outactors
    (if (`self.ActorHasTag` _array_element "1")
      (`self.SetActorHiddenInGame` _array_element _returnvalue)
      (`self.SetActorEnableCollision` _array_element _returnvalue_2)
      (else
        (`self.SetActorHiddenInGame` _array_element _returnvalue_2)
        (`self.SetActorEnableCollision` _array_element _returnvalue))))
  (set `self.activeChannel` (`KismetMathLibrary.SelectInt` 2 1 _returnvalue)))

(event `Key|Tab`
  (params (Key :type "Key Structure"))
  (:`Pressed`
    (`self.disableRGB`)
    (`KismetSystemLibrary.PrintString` "RGB Disabled! (5s)")))

(event `disableRGB`
  (bind _rgb (`self.RGB`))
  (bind _returnvalue (`KismetMathLibrary.SelectFloat` 1.0 0.0 _rgb))
  (bind _camera (`/Game/Core/Char_Player.Camera` (cast `/Game/Core/Char_Player` (`self.K2_GetPawn`) :!pure true)))
  ;[1 1 1] RGB Ability
  (if _rgb
    (set `self.RGB` false)
    (bind _outactors (`GameplayStatics.GetAllActorsWithTag` "RGB"))
    (for _array_element _outactors
      (`self.SetActorHiddenInGame` _array_element false)
      (`self.SetActorEnableCollision` _array_element true))
    (set `CameraComponent.PostProcessSettings` (make `PostProcessSettings` :`ColorSaturation` (`KismetMathLibrary.MakeVector4` _returnvalue _returnvalue _returnvalue _returnvalue)) _camera)
    (`KismetSystemLibrary.PrintString` "Hello")
    (`KismetSystemLibrary.Delay` 5.0)
    (for _array_element_2 _outactors
      (`self.SetActorHiddenInGame` _array_element_2 true)
      (`self.SetActorEnableCollision` _array_element_2 false))
    (set `self.RGB` true)
    (set `CameraComponent.PostProcessSettings` (struct) _camera)))

(fn `setUp`
  (bind _returnvalue (pcsubsystem `EnhancedInputLocalPlayerSubsystem` self))
  (bind _returnvalue_2 (`EnhancedInputSubsystemInterface.GetUserSettings` _returnvalue))
  (bind _returnvalue_3 (`|CreateWidget` "/Game/Widgets/UW_HUD.UW_HUD_C"))
  (set `self.HUD` _returnvalue_3)
  (`self.showHUD`)
  (`/Engine/EditorBlueprintResources/StandardMacros.IsValid` _returnvalue
    (:`Is Valid`
      (`EnhancedInputSubsystemInterface.AddMappingContext` _returnvalue "/Game/Core/Inputs/IMC_Base.IMC_Base" 0 (struct))
      (if (not (`EnhancedInputUserSettings.IsMappingContextRegistered` _returnvalue_2 "/Game/Core/Inputs/IMC_Base.IMC_Base"))
        (`EnhancedInputUserSettings.RegisterInputMappingContext` _returnvalue_2 "/Game/Core/Inputs/IMC_Base.IMC_Base")))))

(fn `UserConstructionScript`)