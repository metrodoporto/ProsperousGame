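; Body cam component that applies a selectable post-process look, such as GoPro, VHS, night or thermal vision and stylized shaders, to a camera.
; InitBodyCam enables custom depth on the character mesh, then picks a warped (fisheye) or unwarped preset, storing it as CurrentSettings.
; Digital Camera also adds an overlay widget.
; Toggle events for night, thermal and B&W thermal vision flip-flop between that preset and CurrentSettings.
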(event `InitBodyCam`
  (params (CameraComponent :type "CameraComponent Object Reference") (CharacterMesh :type "MeshComponent Object Reference"))
  (`PrimitiveComponent.SetRenderCustomDepth` CharacterMesh true)
  (switch `/Game/BodyCam/Enums/E_BodyCamWarp` (`self.BodyCamWarpEnum`)
    (:`NewEnumerator0`
      ;[1 1 1 1 114] With Warp
      (switch `/Game/BodyCam/Enums/E_CameraEffects` (`self.CameraEffects`)
        (:`NewEnumerator3`
          (`self.GoProWithWarp` CameraComponent))
        (:`NewEnumerator0`
          (`self.VHSWithWarp` CameraComponent))
        (:`NewEnumerator1`
          (`self.VHSWarnWithWarp` CameraComponent))
        (:`NewEnumerator2`
          (`self.DigitalCamWithWarp` CameraComponent))
        (:`NewEnumerator4`
          (`self.NightVisionWithWarp` CameraComponent))
        (:`NewEnumerator7`
          (`self.ThermalVisionWithWarp` CameraComponent))
        (:`NewEnumerator8`
          (`self.B&WThermalWithWarp` CameraComponent))
        (:`NewEnumerator9`
          (`self.RetroShaderWithWarp` CameraComponent))
        (:`NewEnumerator10`
          (`self.B&WFilmWithWarp` CameraComponent))
        (:`NewEnumerator11`
          (`self.GlowingOutlineWithWarp` CameraComponent))
        (:`NewEnumerator12`
          (`self.CelShadedWarped` CameraComponent))
        (:`NewEnumerator13`
          (`self.ToonShadingWithWarp` CameraComponent))
        (:`NewEnumerator14`
          (`self.StylizedOutlineWithWarp` CameraComponent))
        (:`NewEnumerator5`
          (set `CameraComponent.PostProcessSettings` (`self.CurrentSettings`) CameraComponent))))
    (:`NewEnumerator1`
      ;[1 1 1 1 66] Without Warp
      (switch `/Game/BodyCam/Enums/E_CameraEffects` (`self.CameraEffects`)
        (:`NewEnumerator3`
          (`self.GoProNoWarp` CameraComponent))
        (:`NewEnumerator0`
          (`self.VHSNoWarp` CameraComponent))
        (:`NewEnumerator1`
          (`self.VHSWarnNoWarp` CameraComponent))
        (:`NewEnumerator2`
          (`self.DigitalCamNoWarp` CameraComponent))
        (:`NewEnumerator4`
          (`self.NightVisionNoWarp` CameraComponent))
        (:`NewEnumerator7`
          (`self.ThermalVisionNoWarp` CameraComponent))
        (:`NewEnumerator8`
          (`self.B&WThermalNoWarp` CameraComponent))
        (:`NewEnumerator9`
          (`self.RetroShaderNoWarp` CameraComponent))
        (:`NewEnumerator10`
          (`self.B&WFilm` CameraComponent))
        (:`NewEnumerator11`
          (`self.GlowingOutlineNoWarp` CameraComponent))
        (:`NewEnumerator12`
          (`self.CelShaded` CameraComponent))
        (:`NewEnumerator13`
          (`self.ToonShadingNoWarp` CameraComponent))
        (:`NewEnumerator14`
          (`self.StylizedOutlineNoWarp` CameraComponent))
        (:`NewEnumerator5`
          (set `CameraComponent.PostProcessSettings` (`self.CurrentSettings`) CameraComponent))))))

(event `ToggleNightVision`
  (params (CameraComponent :type "CameraComponent Object Reference"))
  (switch `/Game/BodyCam/Enums/E_BodyCamWarp` (`self.BodyCamWarpEnum`)
    (:`NewEnumerator0`
      (`/Engine/EditorBlueprintResources/StandardMacros.FlipFlop`
        (:`A`
          (set `CameraComponent.PostProcessSettings` (`self.NightVisionFished`) CameraComponent))
        (:`B`
          (set `CameraComponent.PostProcessSettings` (`self.CurrentSettings`) CameraComponent))))
    (:`NewEnumerator1`
      (`/Engine/EditorBlueprintResources/StandardMacros.FlipFlop`
        (:`A`
          (set `CameraComponent.PostProcessSettings` (`self.NightVision`) CameraComponent))
        (:`B`
          (set `CameraComponent.PostProcessSettings` (`self.CurrentSettings`) CameraComponent))))))

(event `ToggleThermalVision`
  (params (CameraComponent :type "CameraComponent Object Reference"))
  (switch `/Game/BodyCam/Enums/E_BodyCamWarp` (`self.BodyCamWarpEnum`)
    (:`NewEnumerator0`
      (`/Engine/EditorBlueprintResources/StandardMacros.FlipFlop`
        (:`A`
          (set `CameraComponent.PostProcessSettings` (`self.ThermalVisionFished`) CameraComponent))
        (:`B`
          (set `CameraComponent.PostProcessSettings` (`self.CurrentSettings`) CameraComponent))))
    (:`NewEnumerator1`
      (`/Engine/EditorBlueprintResources/StandardMacros.FlipFlop`
        (:`A`
          (set `CameraComponent.PostProcessSettings` (`self.ThermalVision`) CameraComponent))
        (:`B`
          (set `CameraComponent.PostProcessSettings` (`self.CurrentSettings`) CameraComponent))))))

(event `ToggleBlackAndWhiteThermalVision`
  (params (CameraComponent :type "CameraComponent Object Reference"))
  (switch `/Game/BodyCam/Enums/E_BodyCamWarp` (`self.BodyCamWarpEnum`)
    (:`NewEnumerator0`
      (`/Engine/EditorBlueprintResources/StandardMacros.FlipFlop`
        (:`A`
          (set `CameraComponent.PostProcessSettings` (`self.BlackAndWhiteThermalVisionFished`) CameraComponent))
        (:`B`
          (set `CameraComponent.PostProcessSettings` (`self.CurrentSettings`) CameraComponent))))
    (:`NewEnumerator1`
      (`/Engine/EditorBlueprintResources/StandardMacros.FlipFlop`
        (:`A`
          (set `CameraComponent.PostProcessSettings` (`self.BlackAndWhiteThermalVision`) CameraComponent))
        (:`B`
          (set `CameraComponent.PostProcessSettings` (`self.CurrentSettings`) CameraComponent))))))

(fn `B&WFilm`
  (params (CameraComponent :type "CameraComponent Object Reference"))
  (bind _output_get (set `self.CurrentSettings` (`self.BlackAndWhiteFilm`)))
  (set `CameraComponent.PostProcessSettings` _output_get CameraComponent))

(fn `B&WFilmWithWarp`
  (params (CameraComponent :type "CameraComponent Object Reference"))
  (bind _output_get (set `self.CurrentSettings` (`self.BlackAndWhiteFilmFished`)))
  (set `CameraComponent.PostProcessSettings` _output_get CameraComponent))

(fn `B&WThermalNoWarp`
  (params (CameraComponent :type "CameraComponent Object Reference"))
  (bind _output_get (set `self.CurrentSettings` (`self.BlackAndWhiteThermalVision`)))
  (set `CameraComponent.PostProcessSettings` _output_get CameraComponent))

(fn `B&WThermalWithWarp`
  (params (CameraComponent :type "CameraComponent Object Reference"))
  (bind _output_get (set `self.CurrentSettings` (`self.BlackAndWhiteThermalVisionFished`)))
  (set `CameraComponent.PostProcessSettings` _output_get CameraComponent))

(fn `CelShaded`
  (params (CameraComponent :type "CameraComponent Object Reference"))
  (bind _output_get (set `self.CurrentSettings` (`self.CelShader`)))
  (set `CameraComponent.PostProcessSettings` _output_get CameraComponent))

(fn `CelShadedWarped`
  (params (CameraComponent :type "CameraComponent Object Reference"))
  (bind _output_get (set `self.CurrentSettings` (`self.CelShaderFished`)))
  (set `CameraComponent.PostProcessSettings` _output_get CameraComponent))

(fn `DigitalCamNoWarp`
  (params (CameraComponent :type "CameraComponent Object Reference"))
  (bind _returnvalue (`|CreateWidget` "/Game/BodyCam/Overlays/WBP_DigitalCamOverlay.WBP_DigitalCamOverlay_C"))
  (`UserWidget.AddToViewport` _returnvalue 0)
  (bind _output_get (set `self.CurrentSettings` (struct)))
  (set `CameraComponent.PostProcessSettings` _output_get CameraComponent))

(fn `DigitalCamWithWarp`
  (params (CameraComponent :type "CameraComponent Object Reference"))
  (bind _returnvalue (`|CreateWidget` "/Game/BodyCam/Overlays/WBP_DigitalCamOverlay.WBP_DigitalCamOverlay_C"))
  (`UserWidget.AddToViewport` _returnvalue 0)
  (bind _output_get (set `self.CurrentSettings` (`self.FishEye`)))
  (set `CameraComponent.PostProcessSettings` _output_get CameraComponent))

(fn `GlowingOutlineNoWarp`
  (params (CameraComponent :type "CameraComponent Object Reference"))
  (bind _output_get (set `self.CurrentSettings` (`self.GlowingOutline`)))
  (set `CameraComponent.PostProcessSettings` _output_get CameraComponent))

(fn `GlowingOutlineWithWarp`
  (params (CameraComponent :type "CameraComponent Object Reference"))
  (bind _output_get (set `self.CurrentSettings` (`self.GlowingOutlineFished`)))
  (set `CameraComponent.PostProcessSettings` _output_get CameraComponent))

(fn `GoProNoWarp`
  (params (CameraComponent :type "CameraComponent Object Reference"))
  (bind _output_get (set `self.CurrentSettings` (struct)))
  (set `CameraComponent.PostProcessSettings` _output_get CameraComponent))

(fn `GoProWithWarp`
  (params (CameraComponent :type "CameraComponent Object Reference"))
  (bind _output_get (set `self.CurrentSettings` (`self.FishEye`)))
  (set `CameraComponent.PostProcessSettings` _output_get CameraComponent))

(fn `NightVisionNoWarp`
  (params (CameraComponent :type "CameraComponent Object Reference"))
  (bind _output_get (set `self.CurrentSettings` (`self.NightVision`)))
  (set `CameraComponent.PostProcessSettings` _output_get CameraComponent))

(fn `NightVisionWithWarp`
  (params (CameraComponent :type "CameraComponent Object Reference"))
  (bind _output_get (set `self.CurrentSettings` (`self.NightVisionFished`)))
  (set `CameraComponent.PostProcessSettings` _output_get CameraComponent))

(fn `RetroShaderNoWarp`
  (params (CameraComponent :type "CameraComponent Object Reference"))
  (bind _output_get (set `self.CurrentSettings` (`self.RetoShader`)))
  (set `CameraComponent.PostProcessSettings` _output_get CameraComponent))

(fn `RetroShaderWithWarp`
  (params (CameraComponent :type "CameraComponent Object Reference"))
  (bind _output_get (set `self.CurrentSettings` (`self.RetoShaderFished`)))
  (set `CameraComponent.PostProcessSettings` _output_get CameraComponent))

(fn `StylizedOutlineNoWarp`
  (params (CameraComponent :type "CameraComponent Object Reference"))
  (bind _output_get (set `self.CurrentSettings` (`self.StylizedOutline`)))
  (set `CameraComponent.PostProcessSettings` _output_get CameraComponent))

(fn `StylizedOutlineWithWarp`
  (params (CameraComponent :type "CameraComponent Object Reference"))
  (bind _output_get (set `self.CurrentSettings` (`self.StylizedOutlineFished`)))
  (set `CameraComponent.PostProcessSettings` _output_get CameraComponent))

(fn `ThermalVisionNoWarp`
  (params (CameraComponent :type "CameraComponent Object Reference"))
  (bind _output_get (set `self.CurrentSettings` (`self.ThermalVision`)))
  (set `CameraComponent.PostProcessSettings` _output_get CameraComponent))

(fn `ThermalVisionWithWarp`
  (params (CameraComponent :type "CameraComponent Object Reference"))
  (bind _output_get (set `self.CurrentSettings` (`self.ThermalVisionFished`)))
  (set `CameraComponent.PostProcessSettings` _output_get CameraComponent))

(fn `ToonShadingNoWarp`
  (params (CameraComponent :type "CameraComponent Object Reference"))
  (bind _output_get (set `self.CurrentSettings` (`self.ToonOutline`)))
  (set `CameraComponent.PostProcessSettings` _output_get CameraComponent))

(fn `ToonShadingWithWarp`
  (params (CameraComponent :type "CameraComponent Object Reference"))
  (bind _output_get (set `self.CurrentSettings` (`self.ToonOutlinefished`)))
  (set `CameraComponent.PostProcessSettings` _output_get CameraComponent))

(fn `VHSNoWarp`
  (params (CameraComponent :type "CameraComponent Object Reference"))
  (bind _output_get (set `self.CurrentSettings` (`self.VHSNew   `)))
  (set `CameraComponent.PostProcessSettings` _output_get CameraComponent))

(fn `VHSWarnNoWarp`
  (params (CameraCompoent :type "CameraComponent Object Reference"))
  (bind _output_get (set `self.CurrentSettings` (`self.VHSWarnOut`)))
  (set `CameraComponent.PostProcessSettings` _output_get CameraCompoent))

(fn `VHSWarnWithWarp`
  (params (CameraComponent :type "CameraComponent Object Reference"))
  (set `self.CurrentSettings` (`self.VHSWarnOutFished`))
  (set `CameraComponent.PostProcessSettings` (`self.CurrentSettings`) CameraComponent))

(fn `VHSWithWarp`
  (params (CameraComponent :type "CameraComponent Object Reference"))
  (set `self.CurrentSettings` (`self.VHSNewFished`))
  (set `CameraComponent.PostProcessSettings` (`self.CurrentSettings`) CameraComponent))