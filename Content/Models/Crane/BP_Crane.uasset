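; BP_Crane is a configurable crane that carries a BP_Container child actor on a cable.
; UpdateLine maps Distance to spring arm length, RopeLength to container height, and the two rotation variables to crane head and container yaw, then sets the cable end from the container's offset to the root.
; The construction script applies the container material and calls UpdateLine, which also runs every Tick to follow variable changes.
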(event `self.ReceiveTick`
  (params (DeltaSeconds :type "Float (single-precision)"))
  (`self.updateLine`))

(fn `updateLine`
  (bind _container (`self.Container`))
  (set `SpringArmComponent.TargetArmLength` (`self.Distance`) (`self.SpringArm`))
  (`SceneComponent.K2_SetRelativeLocation` _container (`KismetMathLibrary.MakeVector` 0.0 0.0 (* (`self.Rope Length`) -1.0)) false false)
  (`SceneComponent.K2_SetRelativeRotation` _container (`KismetMathLibrary.MakeRotator` 0.0 0.0 (`self.Container Rotation`)) false false)
  (`SceneComponent.K2_SetRelativeRotation` (`self.CraneHead`) (`KismetMathLibrary.MakeRotator` 0.0 0.0 (`self.Rotation`)) false false)
  (set `CableComponent.EndLocation` (- (`SceneComponent.K2_GetComponentLocation` (`self.Container`)) (`SceneComponent.K2_GetComponentLocation` (`self.DefaultSceneRoot`))) (`self.Cable`)))

(fn `UserConstructionScript`
  (set `/Game/Models/Crane/Container/BP_Container.Container Material` (`self.Container Material`) (cast `/Game/Models/Crane/Container/BP_Container` (`ChildActorComponent.ChildActor` (`self.Container`)) :!pure true))
  (`self.updateLine`))