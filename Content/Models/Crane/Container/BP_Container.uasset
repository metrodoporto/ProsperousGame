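; BP_Container is a crane container actor whose Container mesh takes its appearance from a ContainerMaterial variable.
; The construction script applies that material to element 2 of the mesh, and BeginPlay applies it again after a short delay.
; An unconnected debug print of the root's world location remains in the event graph and never runs.
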(event `self.ReceiveBeginPlay`
  (`KismetSystemLibrary.Delay` 0.5)
  (`PrimitiveComponent.SetMaterial` (`self.Container`) 2 (`self.Container Material`)))

(fn `UserConstructionScript`
  (`PrimitiveComponent.SetMaterial` (`self.Container`) 2 (`self.Container Material`)))